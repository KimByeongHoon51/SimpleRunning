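; Game mode for a running race that drives the match through Ready, Play and End phases.
; On BeginPlay it binds to the game state's phase and elapsed-time dispatchers and sets Ready.
; It switches to Play once elapsed time in Ready passes a fixed countdown of about eleven seconds.
; When a character ends the game, it sets End and gives that player one result and all other players another.
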(event EventBeginPlay
  (CallFunction|BindGameState))

(fn ConstructionScript)

(fn BindGameState
  (bind _asbp_running_game_state (Utilities|Casting|CastToBP_RunningGameState (Game|GetGameState)))
  (EventDispatchers|BindEventtoEventDispatcherChangeGameState _asbp_running_game_state (EventDispatchers|CreateEvent :!event UpdateGameState))
  (EventDispatchers|BindEventtoEventDispatcherTotalDeltaSec _asbp_running_game_state (EventDispatchers|CreateEvent :!event UpdateTotalDeltaSec))
  (Default|ChangeGameState _asbp_running_game_state "NewEnumerator1"))

(fn UpdateGameState
  (params (GameState :type EN_GameState%20Enum :default "NewEnumerator0"))
  (Variables|Default|SetGame%20State GameState))

(fn UpdateTotalDeltaSec
  (params (TotalDeltaSec :type Float%20%28double-precision%29))
  (switch Utilities|FlowControl|Switch|SwitchonEN_GameState (Variables|Default|GetGame%20State)
    (:NewEnumerator1
      (if (> TotalDeltaSec 11.0)
        (bind _asbp_running_game_state (Utilities|Casting|CastToBP_RunningGameState (Game|GetGameState)))
        (Default|ChangeGameState _asbp_running_game_state "NewEnumerator2")))))

(fn OnGameEnd
  (params (Character :type Character%20Object%20Reference))
  (bind _asbp_running_game_state (Utilities|Casting|CastToBP_RunningGameState (Game|GetGameState)))
  (Default|ChangeGameState _asbp_running_game_state "NewEnumerator3")
  (CallFunction|UpdateGameResult (Variables|/Script/Engine.Pawn|GetPlayerState Character)))

(fn UpdateGameResult
  (params (PlayerState :type Object%20Object%20Reference))
  (bind _asbp_running_player_state (Utilities|Casting|CastToBP_RunningPlayerState PlayerState))
  (Default|SetGameResult _asbp_running_player_state "NewEnumerator1")
  (bind _outactors (Actor|GetAllActorsOfClass "/Game/Blueprints/Player/BP_RunningPlayerState.BP_RunningPlayerState_C"))
  (for _array_element _outactors
    (if (!= _array_element _asbp_running_player_state)
      (Default|SetGameResult _array_element "NewEnumerator2"))))