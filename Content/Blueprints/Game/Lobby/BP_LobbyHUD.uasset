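; Lobby HUD Blueprint that creates the lobby widget on BeginPlay and refreshes its player list.
; BindPlayerState subscribes to a player state's nickname-change dispatcher and destruction event, and triggers an immediate refresh.
; Nickname changes and the destroy handler both route to UpdateChangeNickName, which calls UpdatePlayerList on the widget.
; If the widget is not yet valid, that update retries on a short timer.
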(event EventBeginPlay
  (bind _returnvalue (UserInterface|CreateWidget "/Game/Blueprints/Widgets/Lobby/LobbyHUDWidget.LobbyHUDWidget_C"))
  (bind _output_get (Variables|Default|SetLobbyHUDWidget _returnvalue))
  (UserInterface|Viewport|AddtoViewport _output_get 0))

(fn ConstructionScript)

(fn BindPlayerState
  (params (PlayerState :type BP%20Lobby%20Player%20State%20Object%20Reference))
  (EventDispatchers|BindEventtoEventDispatcherChangeNickName PlayerState (EventDispatchers|CreateEvent :!event EventChangeNickName))
  (CallFunction|EventChangeNickName (Variables|/Game/Blueprints/Game/Lobby/BP_LobbyPlayerState.BP_LobbyPlayerState_C|GetNickName PlayerState))
  (Game|BindEventtoOnDestroyed PlayerState (EventDispatchers|CreateEvent :!event DestroyNickName)))

(fn EventChangeNickName
  (params (NickName :type String))
  (CallFunction|UpdateChangeNickName))

(fn UpdateChangeNickName
  (bind _lobbyhudwidget (Variables|Default|GetLobbyHUDWidget)
    (:then
      (Default|UpdatePlayerList _lobbyhudwidget))
    (:else
      (Utilities|Time|SetTimerbyFunctionName 0 "UpdateChangeNickName" 0.01))))

(fn DestroyNickName
  (params (DestroyedActor :type Actor%20Object%20Reference))
  (CallFunction|UpdateChangeNickName))